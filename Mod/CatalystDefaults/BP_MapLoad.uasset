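; CatalystDefaults mod blueprint that switches catalyst use on for newly built industries when its mod option is on.
; On load it resolves the building table, retrying on a timer.
; Destroyed construction sites with industry or catalyst rows are queued and polled briefly for the finished actor by class and position; building-spawn events skip the queue.
; It applies the toggle by sending a HUD action through an IndustryDetails widget never added to screen.
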(event Custom|OnBuilt
  (params (Actor :type Actor%20Object%20Reference))
  (bind _returnvalue (Class|ModAPI|ReadModOptionValue (Class|ModAPI|GetModAPI) "CatalystDefaults_On" "On"))
  (if (Utilities|Enum|Equal(Enum) _returnvalue "On")
    (Variables|Default|SetCur Actor)
    (if (Utilities|IsValid (Actor|GetComponentbyClass (Variables|Default|GetCur) "/Script/ProjectArco.Industry"))
      (if (and (Utilities|Name|NotEqual(Name) (Variables|/Script/ProjectArco.Industry|Getm_catalystResource (Actor|GetComponentbyClass (Variables|Default|GetCur) "/Script/ProjectArco.Industry")) "None") (not (Variables|/Script/ProjectArco.Industry|Getm_allowCatalysts (Actor|GetComponentbyClass (Variables|Default|GetCur) "/Script/ProjectArco.Industry"))))
        (if (Utilities|IsValid (Variables|Default|GetView))
          _
          (else
            (bind _returnvalue_2 (UserInterface|CreateWidget "/Script/ProjectArco.IndustryDetails" (Game|GetPlayerController 0)))
            (Variables|Default|SetView _returnvalue_2)))
        (Class|KismetSystemLibrary|SetObjectPropertybyName (Variables|Default|GetView) "Context" (Variables|Default|GetCur))
        (Class|ArcoWidgetBase|ReceiveHudAction (Variables|Default|GetView) (Utilities|Struct|MakeHudAction "setCatalystUse" true))
        (if (Variables|Default|GetDebug)
          (Class|ModAPI|LogMessage (Class|ModAPI|GetModAPI) (Utilities|String|Append (Utilities|String|Append (Utilities|String|Append (Utilities|String|Append (Utilities|String|Append "CatalystDefaults: " "") (Utilities|GetDisplayName (Variables|Default|GetCur))) " Catalyst (") (Utilities|String|ToString(Name) (Variables|/Script/ProjectArco.Industry|Getm_catalystResource (Actor|GetComponentbyClass (Variables|Default|GetCur) "/Script/ProjectArco.Industry")))) ") -> on") true))))))

(event Custom|OnCheck
  (Variables|Default|SetAnyLeft false)
  (for (_array_element _array_index) (Variables|Default|GetPendTries)
    (if (> _array_element 0)
      (Utilities|Array|SetArrayElem (Variables|Default|GetPendTries) _array_index (- _array_element 1))
      (bind _outactors (Actor|GetAllActorsOfClass (Utilities|Array|Get(acopy) (Variables|Default|GetPendClass) _array_index)))
      (for _array_element_2 _outactors
        (bind _asgrid_actor (Utilities|Casting|CastToGridActor _array_element_2))
        (if (or (Utilities|Enum|Equal(Enum) (Utilities|String|ToString(Integer) (Utilities|Struct|BreakGridFootprint (Variables|/Script/ProjectArco.GridActor|GetliveFootprint _asgrid_actor))) (Utilities|Array|Get(acopy) (Variables|Default|GetPendPos) _array_index)) (< (Math|Vector|Distance(Vector) (Transformation|GetActorLocation _array_element_2) (Utilities|Array|Get(acopy) (Variables|Default|GetPendLoc) _array_index)) 1e+01))
          (Utilities|Array|SetArrayElem (Variables|Default|GetPendTries) _array_index -1)
          (Variables|Default|SetCur _array_element_2)
          (if (Utilities|IsValid (Actor|GetComponentbyClass (Variables|Default|GetCur) "/Script/ProjectArco.Industry"))
            (if (and (Utilities|Name|NotEqual(Name) (Variables|/Script/ProjectArco.Industry|Getm_catalystResource (Actor|GetComponentbyClass (Variables|Default|GetCur) "/Script/ProjectArco.Industry")) "None") (not (Variables|/Script/ProjectArco.Industry|Getm_allowCatalysts (Actor|GetComponentbyClass (Variables|Default|GetCur) "/Script/ProjectArco.Industry"))))
              (if (Utilities|IsValid (Variables|Default|GetView))
                _
                (else
                  (bind _returnvalue (UserInterface|CreateWidget "/Script/ProjectArco.IndustryDetails" (Game|GetPlayerController 0)))
                  (Variables|Default|SetView _returnvalue)))
              (Class|KismetSystemLibrary|SetObjectPropertybyName (Variables|Default|GetView) "Context" (Variables|Default|GetCur))
              (Class|ArcoWidgetBase|ReceiveHudAction (Variables|Default|GetView) (Utilities|Struct|MakeHudAction "setCatalystUse" true))
              (if (Variables|Default|GetDebug)
                (Class|ModAPI|LogMessage (Class|ModAPI|GetModAPI) (Utilities|String|Append (Utilities|String|Append (Utilities|String|Append (Utilities|String|Append (Utilities|String|Append "CatalystDefaults: " "") (Utilities|GetDisplayName (Variables|Default|GetCur))) " Catalyst (") (Utilities|String|ToString(Name) (Variables|/Script/ProjectArco.Industry|Getm_catalystResource (Actor|GetComponentbyClass (Variables|Default|GetCur) "/Script/ProjectArco.Industry")))) ") -> on") true))))))
      (if (> (Utilities|Array|Get(acopy) (Variables|Default|GetPendTries) _array_index) 0)
        (Variables|Default|SetAnyLeft true)
        (elif (== (Utilities|Array|Get(acopy) (Variables|Default|GetPendTries) _array_index) 0)
          (if (Variables|Default|GetDebug)
            (Class|ModAPI|LogMessage (Class|ModAPI|GetModAPI) (Utilities|String|Append (Utilities|String|Append (Utilities|String|Append (Utilities|String|Append (Utilities|String|Append "CatalystDefaults: no finished " "") (Utilities|GetClassDisplayName (Utilities|Array|Get(acopy) (Variables|Default|GetPendClass) _array_index))) " found at ") (Utilities|Array|Get(acopy) (Variables|Default|GetPendPos) _array_index)) " (cancelled?)") true))))))
  (if (Variables|Default|GetAnyLeft)
    (Utilities|Time|SetTimerbyFunctionName self "OnCheck" 1.0)
    (else
      (Utilities|Array|Clear (Variables|Default|GetPendClass))
      (Utilities|Array|Clear (Variables|Default|GetPendPos))
      (Utilities|Array|Clear (Variables|Default|GetPendLoc))
      (Utilities|Array|Clear (Variables|Default|GetPendTries)))))

(event Custom|OnConstruction
  (params (Actor :type Actor%20Object%20Reference))
  (Game|BindEventtoOnDestroyed Actor (delegate Custom|OnSiteGone)))

(event Custom|OnLoaded
  (if (not (Variables|Default|GetReady))
    (bind _returnvalue (Class|ModAPI|HasDataTable (Class|ModAPI|GetModAPI) "GridDefsSync"))
    (bind _returnvalue_2 (Class|ModAPI|HasDataTable (Class|ModAPI|GetModAPI) "GridActors"))
    (if (or (or _returnvalue _returnvalue_2) (>= (Variables|Default|GetSetupTries) 10))
      (Variables|Default|SetReady true)
      (bind _returnvalue_3 (Class|ModAPI|ReadModTextFile (Class|ModAPI|GetModAPI) "CatalystDefaultsConfig" "debug"))
      (Variables|Default|SetDebug (not (Utilities|Array|IsEmpty _returnvalue_3)))
      (bind _returnvalue_4 (Class|ModAPI|HasDataTable (Class|ModAPI|GetModAPI) "GridDefsSync"))
      (if _returnvalue_4
        (Variables|Default|SetTableName "GridDefsSync")
        (if (Variables|Default|GetDebug)
          (Class|ModAPI|LogMessage (Class|ModAPI|GetModAPI) "CatalystDefaults ready (table GridDefsSync)" true))
        (else
          (bind _returnvalue_5 (Class|ModAPI|HasDataTable (Class|ModAPI|GetModAPI) "GridActors"))
          (if _returnvalue_5
            (Variables|Default|SetTableName "GridActors")
            (if (Variables|Default|GetDebug)
              (Class|ModAPI|LogMessage (Class|ModAPI|GetModAPI) "CatalystDefaults ready (table GridActors)" true))
            (else
              (if (Variables|Default|GetDebug)
                (Class|ModAPI|LogMessage (Class|ModAPI|GetModAPI) "CatalystDefaults: building table not found - mod inactive. Tables the mod API knows:" true))
              (bind _returnvalue_6 (Class|ModAPI|ListDataTables (Class|ModAPI|GetModAPI)))
              (for _array_element _returnvalue_6
                (if (Variables|Default|GetDebug)
                  (Class|ModAPI|LogMessage (Class|ModAPI|GetModAPI) (Utilities|String|Append (Utilities|String|Append "CatalystDefaults:   table " "") (Utilities|String|ToString(Name) _array_element)) true)))))))
      (else
        (Variables|Default|SetSetupTries (+ (Variables|Default|GetSetupTries) 1))
        (Utilities|Time|SetTimerbyFunctionName self "OnLoaded" 1.0)))))

(event Custom|OnSiteGone
  (params (DestroyedActor :type Actor%20Object%20Reference))
  (bind _returnvalue (Actor|GetComponentbyClass DestroyedActor "/Script/ProjectArco.ConstructionSite"))
  (bind _tablename (Variables|Default|GetTableName))
  (bind _m_gridactortobuild (Variables|/Script/ProjectArco.ConstructionSite|Getm_gridActorToBuild _returnvalue))
  (bind _returnvalue_2 (Class|ModAPI|ReadModOptionValue (Class|ModAPI|GetModAPI) "CatalystDefaults_On" "On"))
  (if (and (Utilities|Enum|Equal(Enum) _returnvalue_2 "On") (Utilities|IsValid _returnvalue))
    (bind _returnvalue_3 (Class|ModAPI|ReadDataTableValue (Class|ModAPI|GetModAPI) _tablename _m_gridactortobuild "asIndustryDef"))
    (bind _returnvalue_4 (Class|ModAPI|ReadDataTableValue (Class|ModAPI|GetModAPI) _tablename _m_gridactortobuild "catalyst"))
    (if (or (and (not (Utilities|Array|IsEmpty _returnvalue_3)) (Utilities|Enum|NotEqual(Enum) _returnvalue_3 "None")) (and (not (Utilities|Array|IsEmpty _returnvalue_4)) (Utilities|Enum|NotEqual(Enum) _returnvalue_4 "None")))
      (bind _returnvalue_5 (Class|ModAPI|ReadDataTableValue (Class|ModAPI|GetModAPI) _tablename _m_gridactortobuild "GridActor"))
      (bind _returnvalue_6 (Utilities|LoadClassAssetBlocking (Class|KismetSystemLibrary|ToSoftClassRef(SoftClassPath) (Class|KismetSystemLibrary|MakeSoftClassPath _returnvalue_5))))
      (bind _asactor (Utilities|Casting|CastToActorClass _returnvalue_6)
        (:then
          (bind _asgrid_actor (Utilities|Casting|CastToGridActor DestroyedActor))
          (Utilities|Array|Add (Variables|Default|GetPendClass) _asactor)
          (Utilities|Array|Add (Variables|Default|GetPendPos) (Utilities|String|ToString(Integer) (Utilities|Struct|BreakGridFootprint (Variables|/Script/ProjectArco.GridActor|GetliveFootprint _asgrid_actor))))
          (Utilities|Array|Add (Variables|Default|GetPendLoc) (Transformation|GetActorLocation DestroyedActor))
          (Utilities|Array|Add (Variables|Default|GetPendTries) 4)
          (if (Variables|Default|GetDebug)
            (Class|ModAPI|LogMessage (Class|ModAPI|GetModAPI) (Utilities|String|Append (Utilities|String|Append (Utilities|String|Append (Utilities|String|Append "CatalystDefaults: construction of " "") (Utilities|String|ToString(Name) _m_gridactortobuild)) " ended at ") (Utilities|String|ToString(Integer) (Utilities|Struct|BreakGridFootprint (Variables|/Script/ProjectArco.GridActor|GetliveFootprint _asgrid_actor)))) true))
          (if (not (Class|KismetSystemLibrary|IsTimerActive self "OnCheck"))
            (Utilities|Time|SetTimerbyFunctionName self "OnCheck" 1.0)))
        (:CastFailed
          (if (Variables|Default|GetDebug)
            (Class|ModAPI|LogMessage (Class|ModAPI|GetModAPI) (Utilities|String|Append (Utilities|String|Append "CatalystDefaults: no class for " "") _returnvalue_5) true)))))))

(event EventBeginPlay
  (bind _returnvalue (Class|ModAPI|GetModAPI))
  (EventDispatchers|BindEventtoOnConstructionSpawned _returnvalue (delegate Custom|OnConstruction))
  (EventDispatchers|BindEventtoOnBuildingSpawned _returnvalue (delegate Custom|OnBuilt))
  (EventDispatchers|BindEventtoOnLoadingFinished _returnvalue (delegate Custom|OnLoaded))
  (if (not (Variables|Default|GetReady))
    (bind _returnvalue_2 (Class|ModAPI|HasDataTable (Class|ModAPI|GetModAPI) "GridDefsSync"))
    (bind _returnvalue_3 (Class|ModAPI|HasDataTable (Class|ModAPI|GetModAPI) "GridActors"))
    (if (or (or _returnvalue_2 _returnvalue_3) (>= (Variables|Default|GetSetupTries) 10))
      (Variables|Default|SetReady true)
      (bind _returnvalue_4 (Class|ModAPI|ReadModTextFile (Class|ModAPI|GetModAPI) "CatalystDefaultsConfig" "debug"))
      (Variables|Default|SetDebug (not (Utilities|Array|IsEmpty _returnvalue_4)))
      (bind _returnvalue_5 (Class|ModAPI|HasDataTable (Class|ModAPI|GetModAPI) "GridDefsSync"))
      (if _returnvalue_5
        (Variables|Default|SetTableName "GridDefsSync")
        (if (Variables|Default|GetDebug)
          (Class|ModAPI|LogMessage (Class|ModAPI|GetModAPI) "CatalystDefaults ready (table GridDefsSync)" true))
        (else
          (bind _returnvalue_6 (Class|ModAPI|HasDataTable (Class|ModAPI|GetModAPI) "GridActors"))
          (if _returnvalue_6
            (Variables|Default|SetTableName "GridActors")
            (if (Variables|Default|GetDebug)
              (Class|ModAPI|LogMessage (Class|ModAPI|GetModAPI) "CatalystDefaults ready (table GridActors)" true))
            (else
              (if (Variables|Default|GetDebug)
                (Class|ModAPI|LogMessage (Class|ModAPI|GetModAPI) "CatalystDefaults: building table not found - mod inactive. Tables the mod API knows:" true))
              (bind _returnvalue_7 (Class|ModAPI|ListDataTables (Class|ModAPI|GetModAPI)))
              (for _array_element _returnvalue_7
                (if (Variables|Default|GetDebug)
                  (Class|ModAPI|LogMessage (Class|ModAPI|GetModAPI) (Utilities|String|Append (Utilities|String|Append "CatalystDefaults:   table " "") (Utilities|String|ToString(Name) _array_element)) true)))))))
      (else
        (Variables|Default|SetSetupTries (+ (Variables|Default|GetSetupTries) 1))
        (Utilities|Time|SetTimerbyFunctionName self "OnLoaded" 1.0)))))

(fn ConstructionScript)